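; BP_Acid is a damaging acid hazard that hurts the first-person player character while they stand inside its box volume.
; On begin overlap it stores the player and starts a looping timer that applies a configurable damage amount at each configurable interval.
; When the character leaves the box, the stored timer handle is cleared to stop the damage.
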(event `self.Box.OnComponentBeginOverlap`
  (params (OverlappedComponent :type "PrimitiveComponent Object Reference") (OtherActor :type "Actor Object Reference") (OtherComp :type "PrimitiveComponent Object Reference") (OtherBodyIndex :type Integer) (bFromSweep :type Boolean) (SweepResult :type "HitResult Structure (by ref)"))
  (bind _asbp_first_person_character (cast `/Game/FirstPerson/Blueprints/BP_FirstPersonCharacter` OtherActor))
  (set `self.Player` _asbp_first_person_character)
  (bind _returnvalue (`KismetSystemLibrary.K2_SetTimerDelegate` (delegate `AcidTimer`) (`self.AcidTime`) true))
  (set `self.Acid` _returnvalue))

(event `AcidTimer`
  (`GameplayStatics.ApplyDamage` (`self.Player`) (`self.Damage`)))

(event `self.Box.OnComponentEndOverlap`
  (params (OverlappedComponent :type "PrimitiveComponent Object Reference") (OtherActor :type "Actor Object Reference") (OtherComp :type "PrimitiveComponent Object Reference") (OtherBodyIndex :type Integer))
  (cast `/Game/FirstPerson/Blueprints/BP_FirstPersonCharacter` OtherActor)
  (`KismetSystemLibrary.K2_ClearAndInvalidateTimerHandle` (`self.Acid`)))

(fn `UserConstructionScript`)