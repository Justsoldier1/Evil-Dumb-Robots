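; BP_SanitizerGrenade is a sanitizer grenade actor that deals direct and splash damage on impact.
; When its Collision component hits, it damages the struck actor, then runs a zero-length multi-sphere object trace at the Sanitizer component's location.
; Each trace hit receives splash damage and, if the actor is valid, a BP_Bubble spawned at its transform.
; The grenade then destroys itself.
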(event `self.Collision.OnComponentHit`
  (params (HitComponent :type "PrimitiveComponent Object Reference") (OtherActor :type "Actor Object Reference") (OtherComp :type "PrimitiveComponent Object Reference") (NormalImpulse :type "Vector Structure") (Hit :type "HitResult Structure (by ref)"))
  (bind _returnvalue (`SceneComponent.K2_GetComponentLocation` (`self.Sanitizer`)))
  ;[1 1 1] Hit
  (`GameplayStatics.ApplyDamage` OtherActor (`self.Direct Damage`))
  ;[1 1 1] Splash Damage
  (bind _outhits (`KismetSystemLibrary.SphereTraceMultiForObjects` _returnvalue _returnvalue (`self.ExplosionSize`) (`self.Object Types`)))
  (for _array_element _outhits
    (bind (_bblockinghit _binitialoverlap _time _distance _location _impactpoint _normal _impactnormal _physmat _hitactor) (`GameplayStatics.BreakHitResult` _array_element))
    (`GameplayStatics.ApplyDamage` _hitactor (`self.SplashDamage`))
    (`/Engine/EditorBlueprintResources/StandardMacros.IsValid` _hitactor
      (:`Is Valid`
        (`|SpawnActorFromClass` "/Game/Blueprints/BP_Bubble.BP_Bubble_C" (`KismetMathLibrary.MakeTransform` (`self.K2_GetActorLocation` _hitactor) (`self.K2_GetActorRotation` _hitactor)) "Undefined" "MultiplyWithRoot" null null))))
  (`self.K2_DestroyActor`))

(fn `UserConstructionScript`)