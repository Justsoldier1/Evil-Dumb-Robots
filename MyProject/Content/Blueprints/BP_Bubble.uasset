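; BP_Bubble is a projectile bubble that damages and traps whatever actor overlaps its sphere, treated as an enemy.
; A looping timer keeps teleporting the caught actor to the bubble and applies a set projectile gravity, popping once that actor becomes invalid.
; Taking any damage also pops it: a fast timer shrinks the bubble in steps, then spawns a Niagara pop effect and destroys it.
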(event `self.ReceiveAnyDamage`
  (params (Damage :type "Float (single-precision)") (DamageType :type "DamageType Object Reference") (InstigatedBy :type "Controller Object Reference") (DamageCauser :type "Actor Object Reference"))
  ;[1 1 1] Popping
  (`self.Pop`))

(event `Pop`
  ;[1 1 1] Popping
  (`KismetSystemLibrary.K2_SetTimerDelegate` (delegate `Dead`) 0.01 true))

(event `Dead`
  (bind _returnvalue (+ (`self.ScaleIncrement`) 1))
  ;[1 1 1] Popping
  (`self.SetActorScale3D` (- (`self.GetActorScale3D`) (0.1 0.1 0.1)))
  (set `self.ScaleIncrement` _returnvalue)
  (if (>= _returnvalue 10)
    (`NiagaraFunctionLibrary.SpawnSystemAtLocation` "/Game/Emitters/NS_BubblePop.NS_BubblePop" (`self.K2_GetActorLocation`))
    (`self.K2_DestroyActor`)))

(event `self.Sphere.OnComponentBeginOverlap`
  (params (OverlappedComponent :type "PrimitiveComponent Object Reference") (OtherActor :type "Actor Object Reference") (OtherComp :type "PrimitiveComponent Object Reference") (OtherBodyIndex :type Integer) (bFromSweep :type Boolean) (SweepResult :type "HitResult Structure (by ref)"))
  ;[1 1 1] TrappingEnemies
  (bind _output_get (set `self.CaughtEnemy` OtherActor))
  (`GameplayStatics.ApplyDamage` _output_get (`self.BaseDamage`))
  (if (not (`self.EnemyInside`))
    (`KismetSystemLibrary.K2_SetTimerDelegate` (delegate `GotEnemy`) 0.01 true)))

(event `GotEnemy`
  ;[1 1 1] TrappingEnemies
  (`/Engine/EditorBlueprintResources/StandardMacros.IsValid` (`self.CaughtEnemy`)
    (:`Is Valid`
      (set `self.EnemyInside` true)
      (`self.K2_SetActorLocation` (`self.CaughtEnemy`) (+ (`self.K2_GetActorLocation`) (`self.GetActorUpVector`)) false false)
      (set `ProjectileMovementComponent.ProjectileGravityScale` (`self.Gravity`) (`self.ProjectileMovement`)))
    (:`Is Not Valid`
      (`self.Pop`))))

(fn `UserConstructionScript`)