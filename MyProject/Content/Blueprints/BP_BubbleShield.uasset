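; BP_BubbleShield is a bubble shield actor that follows the player and pops when it takes any damage.
; A looping 0.01-second timer started on BeginPlay snaps it to the first player character's location.
; Its collision overlap caches the BP_FirstPersonCharacter reference.
; On damage, it clears HasShield, sets that character's NotInBubble flag to true and destroys itself.
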(event `self.ReceiveAnyDamage`
  (params (Damage :type "Float (single-precision)") (DamageType :type "DamageType Object Reference") (InstigatedBy :type "Controller Object Reference") (DamageCauser :type "Actor Object Reference"))
  ;[1 1 1] Pop
  (set `self.HasShield` false)
  (set `/Game/FirstPerson/Blueprints/BP_FirstPersonCharacter.NotInBubble` true (`self.PlayerReference`))
  (`self.K2_DestroyActor`))

(event `self.ReceiveBeginPlay`
  ;[1 1 1] Follow Player
  (set `self.HasShield` true)
  (`KismetSystemLibrary.K2_SetTimerDelegate` (delegate `FollowPlayer`) 0.01 true))

(event `FollowPlayer`
  (bind _returnvalue (`GameplayStatics.GetPlayerCharacter` 0))
  ;[1 1 1] Follow Player
  (`/Engine/EditorBlueprintResources/StandardMacros.IsValid` _returnvalue
    (:`Is Valid`
      (`self.K2_SetActorLocation` (`self.K2_GetActorLocation` _returnvalue)))))

(event `self.Collision.OnComponentBeginOverlap`
  (params (OverlappedComponent :type "PrimitiveComponent Object Reference") (OtherActor :type "Actor Object Reference") (OtherComp :type "PrimitiveComponent Object Reference") (OtherBodyIndex :type Integer) (bFromSweep :type Boolean) (SweepResult :type "HitResult Structure (by ref)"))
  ;[1 1 1] Finding Player
  (bind _asbp_first_person_character (cast `/Game/FirstPerson/Blueprints/BP_FirstPersonCharacter` OtherActor))
  (set `self.PlayerReference` _asbp_first_person_character))

(fn `UserConstructionScript`)