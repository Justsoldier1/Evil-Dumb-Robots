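; Enemy germ-bomb grenade that explodes on hit, dealing direct damage to the struck actor, spawning a gunk Niagara burst and destroying itself.
; Two multi-sphere traces at the bomb's location find a surface for a temporary germ decal and targets for splash damage within ExplosionSize.
; Both trace loops have empty bodies, so decal and splash damage run after completion, affecting only the last hit of each trace.
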(event `self.Collision.OnComponentHit`
  (params (HitComponent :type "PrimitiveComponent Object Reference") (OtherActor :type "Actor Object Reference") (OtherComp :type "PrimitiveComponent Object Reference") (NormalImpulse :type "Vector Structure") (Hit :type "HitResult Structure (by ref)"))
  (bind _returnvalue (`SceneComponent.K2_GetComponentLocation` (`self.GermBomb`)))
  (bind _returnvalue_2 (`SceneComponent.K2_GetComponentLocation` (`self.GermBomb`)))
  ;[1 1 1] Hit
  (`GameplayStatics.ApplyDamage` OtherActor (`self.Direct Damage`))
  ;[1 1 1] Niagra
  (`NiagaraFunctionLibrary.SpawnSystemAtLocation` "/Game/Emitters/NS_GunkExplosion.NS_GunkExplosion" (`SceneComponent.K2_GetComponentLocation` (`self.GermBomb`)))
  ;[1 1 1] Decal
  (bind _outhits (`KismetSystemLibrary.SphereTraceMultiForObjects` _returnvalue _returnvalue 200.0 (`self.Object Types_0`)))
  (for _array_element _outhits
    _)
  (bind (_bblockinghit _binitialoverlap _time _distance _location _impactpoint _normal) (`GameplayStatics.BreakHitResult` _array_element))
  (`GameplayStatics.SpawnDecalAtLocation` "/Game/Decals/M_GermSlash.M_GermSlash" (300.0 300.0 300.0) _location (`KismetMathLibrary.Conv_VectorToRotator` _normal) 10.0)
  ;[1 1 1] Splash Damage
  (bind _outhits_2 (`KismetSystemLibrary.SphereTraceMultiForObjects` _returnvalue_2 _returnvalue_2 (`self.ExplosionSize`) (`self.Object Types`)))
  (for _array_element_2 _outhits_2
    _)
  (`GameplayStatics.ApplyDamage` (`.HitActor` (`GameplayStatics.BreakHitResult` _array_element_2)) (`self.SplashDamage`))
  (`self.K2_DestroyActor`))

(fn `UserConstructionScript`)