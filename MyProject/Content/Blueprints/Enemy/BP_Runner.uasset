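; BP_Runner is an enemy that patrols around a BP_RunnerBase and intermittently charges the player.
; A sphere trace on BeginPlay and detection-sphere overlaps set its base; movement picks random navigable points around it while patrolling.
; A looping run timer randomly interrupts patrol to AI-move to the player.
; On arrival, a small sphere trace applies damage to hit actors, and patrolling resumes.
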(event `self.Movement`
  (bind _base (`self.Base`))
  ;[1 1 1] Moving around base
  (if (`self.Patrolling`)
    (`/Engine/EditorBlueprintResources/StandardMacros.IsValid` _base
      (:`Is Valid`
        (bind _randomlocation (`NavigationSystemV1.K2_GetRandomLocationInNavigableRadius` (`self.K2_GetActorLocation` _base) 400.0 null null))
        (`|AIMoveTo` self _randomlocation null)))))

(event `StartRunTimer`
  ;[1 1 1] RunTimer
  (bind _returnvalue (`KismetSystemLibrary.K2_SetTimerDelegate` (delegate `RunChance`) (`self.RunInterval`) true))
  (set `self.RunTimer` _returnvalue))

(event `self.ReceiveBeginPlay`
  (bind _returnvalue (`self.K2_GetActorLocation`))
  ;[1 1 1] FindBase
  (bind _outhits (`KismetSystemLibrary.SphereTraceMultiForObjects` _returnvalue _returnvalue 600.0 (`self.Object Types`)))
  (for _array_element _outhits
    (bind _asbp_runner_base (cast `/Game/Blueprints/Enemy/BP_RunnerBase` (`.HitActor` (`GameplayStatics.BreakHitResult` _array_element))))
    (set `self.Base` _asbp_runner_base)
    (`self.StartMovementTimer`)
    (`self.StartRunTimer` :!label _label))
  (goto _label))

(event `RunChance`
  (bind _returnvalue (`self.K2_GetActorLocation`))
  ;[1 1 1] RunChance
  (if (`KismetMathLibrary.RandomBool`)
    (set `self.Patrolling` false)
    (`|AIMoveTo` self (0.0 0.0 0.0) (`self.Player`) 50.0
      (:`OnSuccess`
        (bind _outhits (`KismetSystemLibrary.SphereTraceMultiForObjects` _returnvalue _returnvalue 60.0 (`self.Object Types_0`)))
        (for _array_element _outhits
          (`GameplayStatics.ApplyDamage` (`.HitActor` (`GameplayStatics.BreakHitResult` _array_element)) (`self.Damage`)))
        (set `self.Patrolling` true)))))

(event `self.DetectionSphere.OnComponentBeginOverlap`
  (params (OverlappedComponent :type "PrimitiveComponent Object Reference") (OtherActor :type "Actor Object Reference") (OtherComp :type "PrimitiveComponent Object Reference") (OtherBodyIndex :type Integer) (bFromSweep :type Boolean) (SweepResult :type "HitResult Structure (by ref)"))
  ;[1 1 1] Detecting base
  (bind _asbp_runner_base (cast `/Game/Blueprints/Enemy/BP_RunnerBase` OtherActor))
  (set `self.Base` _asbp_runner_base))

(fn `UserConstructionScript`
  (`parent.UserConstructionScript`))