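; BP_Roller is an enemy Blueprint with custom Movement and Attack events.
; Movement uses AI MoveTo to approach the Player, then, on success, prints a debug message and moves to a random navigable point near its own location.
; Attack spawns a BP_EnemyProjectile at the location and rotation of its Arrow1 component.
; Neither event is called within this graph, and the construction script only runs the parent's.
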(event `self.Movement`
  ;[1 1 1] Movement
  (`|AIMoveTo` self (0.0 0.0 0.0) (`self.Player`) 250.0
    (:`OnSuccess`
      (`KismetSystemLibrary.PrintString` "Done")
      (bind _randomlocation (`NavigationSystemV1.K2_GetRandomLocationInNavigableRadius` (`self.K2_GetActorLocation`) 250.0 null null))
      (`|AIMoveTo` self _randomlocation null))))

(event `self.Attack`
  (bind _arrow1 (`self.Arrow1`))
  (`|SpawnActorFromClass` "/Game/Blueprints/Enemy/BP_EnemyProjectile.BP_EnemyProjectile_C" (`KismetMathLibrary.MakeTransform` (`SceneComponent.K2_GetComponentLocation` _arrow1) (`SceneComponent.K2_GetComponentRotation` _arrow1)) "Undefined" "MultiplyWithRoot" null null))

(fn `UserConstructionScript`
  (`parent.UserConstructionScript`))