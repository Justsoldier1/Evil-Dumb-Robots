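; Wave manager that spawns endless waves of enemies around itself, starting on BeginPlay.
; Each wave increments WaveNumber, resets EnemyCount and spawns a fixed-size batch of random bacilli, roller, runner or summoner enemies at reachable navmesh points within a radius.
; A looping timer polls EnemyCount and starts the next wave at zero; nothing in this graph decrements the count.
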(event `self.ReceiveBeginPlay`
  ;[1 1 1] Spawn Wave
  (`self.SpawnWave`)
  (`self.StartChecking`))

(event `SpawnWave`
  (bind _randomlocation (`NavigationSystemV1.K2_GetRandomReachablePointInRadius` (`self.K2_GetActorLocation`) 3000.0 null null))
  ;[1 1 1] Spawn Wave
  (set `self.WaveNumber` (+ (`self.WaveNumber`) 1))
  (for _ (range 10)
    (set `self.EnemyCount` 10)
    (switch `int` (`KismetMathLibrary.RandomIntegerInRange` 0 3)
      (:`0`
        (`|SpawnActorFromClass` "/Game/Blueprints/Enemy/BP_Bacilli1.BP_Bacilli1_C" (`KismetMathLibrary.MakeTransform` _randomlocation) "Undefined" "MultiplyWithRoot" null null))
      (:`1`
        (`|SpawnActorFromClass` "/Game/Blueprints/Enemy/BP_Roller.BP_Roller_C" (`KismetMathLibrary.MakeTransform` _randomlocation) "Undefined" "MultiplyWithRoot" null null))
      (:`2`
        (`|SpawnActorFromClass` "/Game/Blueprints/Enemy/BP_Runner.BP_Runner_C" (`KismetMathLibrary.MakeTransform` _randomlocation) "Undefined" "MultiplyWithRoot" null null))
      (:`3`
        (`|SpawnActorFromClass` "/Game/Blueprints/Enemy/BP_SummonerEnemy.BP_SummonerEnemy_C" (`KismetMathLibrary.MakeTransform` _randomlocation) "Undefined" "MultiplyWithRoot" null null)))))

(event `StartChecking`
  ;[1 1 1] Checking if enemies are dead
  (`KismetSystemLibrary.K2_SetTimerDelegate` (delegate `CheckCount`) 5.0 true))

(event `CheckCount`
  ;[1 1 1] Checking if enemies are dead
  (if (<= (`self.EnemyCount`) 0)
    (`self.SpawnWave`)))

(fn `UserConstructionScript`)