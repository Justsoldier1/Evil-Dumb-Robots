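; Runner base that acts as a healing station for BP_Runner actors within its area.
; Entering the collision volume stores the runner and starts a looping timer that applies HealAmmount through ApplyDamage, and leaving clears that timer.
; BeginPlay runs a sphere trace at the Pool, with persistent debug drawing, to start healing runners already nearby.
; Only one runner reference and timer handle are stored, so each new detection overwrites the previous one.
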(event `self.Collision.OnComponentBeginOverlap`
  (params (OverlappedComponent :type "PrimitiveComponent Object Reference") (OtherActor :type "Actor Object Reference") (OtherComp :type "PrimitiveComponent Object Reference") (OtherBodyIndex :type Integer) (bFromSweep :type Boolean) (SweepResult :type "HitResult Structure (by ref)"))
  ;[1 1 1] Find Runner
  (bind _asbp_runner (cast `/Game/Blueprints/Enemy/BP_Runner` OtherActor))
  (set `self.Runner` _asbp_runner)
  (`self.StartHeal`))

(event `StartHeal`
  ;[1 1 1] Heal Runner
  (bind _returnvalue (`KismetSystemLibrary.K2_SetTimerDelegate` (delegate `HealRunner`) 0.5 true))
  (set `self.HealTimerVariable` _returnvalue))

(event `HealRunner`
  ;[1 1 1] Heal Runner
  (`GameplayStatics.ApplyDamage` (`self.Runner`) (`self.HealAmmount`)))

(event `self.Collision.OnComponentEndOverlap`
  (params (OverlappedComponent :type "PrimitiveComponent Object Reference") (OtherActor :type "Actor Object Reference") (OtherComp :type "PrimitiveComponent Object Reference") (OtherBodyIndex :type Integer))
  ;[1 1 1] Lost Runner
  (cast `/Game/Blueprints/Enemy/BP_Runner` OtherActor)
  (`KismetSystemLibrary.K2_ClearAndInvalidateTimerHandle` (`self.HealTimerVariable`)))

(event `self.ReceiveBeginPlay`
  (bind _returnvalue (`SceneComponent.K2_GetComponentLocation` (`self.Pool`)))
  ;[1 1 1] Find Runner at the start of the game
  (bind _outhits (`KismetSystemLibrary.SphereTraceMultiForObjects` :`Start` _returnvalue :`End` _returnvalue :`Radius` 500.0 :`ObjectTypes` (`self.Object Types`) :`DrawDebugType` "Persistent"))
  (for _array_element _outhits
    (bind _asbp_runner (cast `/Game/Blueprints/Enemy/BP_Runner` (`.HitActor` (`GameplayStatics.BreakHitResult` _array_element))))
    (set `self.Runner` _asbp_runner)
    (`self.StartHeal`)))

(fn `UserConstructionScript`)