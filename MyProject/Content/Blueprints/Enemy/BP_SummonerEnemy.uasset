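; Summoner enemy that wanders the navmesh, tracks the player with its eye and attacks on a timer.
; Looping timers drive aiming, movement and attacks, each attack randomly spawning a group of bacilli nearby or firing a grenade.
; Overlapping its bubble collision blocks damage, new moves and summoning, but not grenades.
; Falling for over half a second sets fall damage, applied on landing.
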(event `LookAtPlayer`
  ;[1 1 1] Look at player
  (`SceneComponent.K2_SetWorldRotation` (`self.Eye`) (`KismetMathLibrary.FindLookAtRotation` (`SceneComponent.K2_GetComponentLocation` (`self.FireArrow`)) (`SceneComponent.K2_GetComponentLocation` (`Character.CapsuleComponent` (`GameplayStatics.GetPlayerCharacter` 0)))) false false))

(event `Attack`
  (bind _spawnrotation (`self.SpawnRotation`))
  (bind _firearrow (`self.FireArrow`))
  ;[1 1 1] Summoning
  (if (`KismetMathLibrary.RandomBool`)
    (if (not (`self.InBubble`))
      (set `self.IsAttacking` true)
      (for _ (range 6)
        (bind _randomlocation (`NavigationSystemV1.K2_GetRandomLocationInNavigableRadius` (`SceneComponent.K2_GetComponentLocation` _spawnrotation) 200.0 null null))
        (`|SpawnActorFromClass` "/Game/Blueprints/Enemy/BP_Bacilli1.BP_Bacilli1_C" (`KismetMathLibrary.MakeTransform` _randomlocation (`SceneComponent.K2_GetComponentRotation` _spawnrotation)) "Undefined" "MultiplyWithRoot" null null))
      (set `self.IsAttacking` false))
    (else
      (`|SpawnActorFromClass` "/Game/Blueprints/Enemy/BP_EnemyGrenade.BP_EnemyGrenade_C" (`KismetMathLibrary.MakeTransform` (`SceneComponent.K2_GetComponentLocation` _firearrow) (`SceneComponent.K2_GetComponentRotation` _firearrow)) "Undefined" "MultiplyWithRoot" null null))))

(event `self.ReceiveBeginPlay`
  ;[1 1 1] Movement
  (bind _returnvalue (`KismetSystemLibrary.K2_SetTimerDelegate` (delegate `Movement`) (`self.MovementSpeed`) true))
  (set `self.MovementTimer` _returnvalue)
  ;[1 1 1] Summoning
  (bind _returnvalue_2 (`KismetSystemLibrary.K2_SetTimerDelegate` (delegate `LookAtPlayer`) 0.1 true))
  (set `self.LookAtPlayerVariable` _returnvalue_2)
  (bind _returnvalue_3 (`KismetSystemLibrary.K2_SetTimerDelegate` (delegate `Attack`) (`self.Attacktime`) true))
  (set `self.AttackTimer` _returnvalue_3))

(event `Movement`
  ;[1 1 1] Movement
  (if (not (`self.IsAttacking`))
    (bind _randomlocation (`NavigationSystemV1.K2_GetRandomLocationInNavigableRadius` (`self.K2_GetActorLocation`) 600.0 null null))
    (if (not (`self.InBubble`))
      (`|AIMoveTo` self _randomlocation null))))

(event `self.ReceiveAnyDamage`
  (params (Damage :type "Float (single-precision)") (DamageType :type "DamageType Object Reference") (InstigatedBy :type "Controller Object Reference") (DamageCauser :type "Actor Object Reference"))
  ;[1 1 1] Damage
  (if (not (`self.InBubble`))
    (bind _output_get (set `self.Health` (- (`self.Health`) Damage)))
    (if (<= _output_get 0.0)
      (`self.K2_DestroyActor`))))

(event `self.BubbleCollision.OnComponentBeginOverlap`
  (params (OverlappedComponent :type "PrimitiveComponent Object Reference") (OtherActor :type "Actor Object Reference") (OtherComp :type "PrimitiveComponent Object Reference") (OtherBodyIndex :type Integer) (bFromSweep :type Boolean) (SweepResult :type "HitResult Structure (by ref)"))
  ;[1 1 1] InBubble
  (set `self.InBubble` true))

(event `self.BubbleCollision.OnComponentEndOverlap`
  (params (OverlappedComponent :type "PrimitiveComponent Object Reference") (OtherActor :type "Actor Object Reference") (OtherComp :type "PrimitiveComponent Object Reference") (OtherBodyIndex :type Integer))
  ;[1 1 1] InBubble
  (set `self.InBubble` false))

(event `self.OnLanded`
  (params (Hit :type "HitResult Structure (by ref)"))
  ;[1 1 1] Apply FallDamage
  (`GameplayStatics.ApplyDamage` self (`self.Falldamage`)))

(event `self.K2_OnMovementModeChanged`
  (params (PrevMovementMode :type "EMovementMode Enum" :default "MOVE_None") (NewMovementMode :type "EMovementMode Enum" :default "MOVE_None") (PrevCustomMode :type Byte) (NewCustomMode :type Byte))
  ;[1 1 1] Calculate FallDamage
  (if (`|EnumEquality` NewMovementMode "MOVE_Falling")
    (`KismetSystemLibrary.RetriggerableDelay` 0.5)
    (if (`NavMovementComponent.IsFalling` (`self.CharacterMovement`))
      (set `self.Falldamage` 2.5))))

(fn `UserConstructionScript`)