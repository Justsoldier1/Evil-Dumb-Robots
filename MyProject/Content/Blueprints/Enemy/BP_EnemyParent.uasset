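; Base enemy Blueprint that detects the first-person player, runs timed movement and attack behavior, and takes damage.
; When the player character enters DetectionSphere, it stores the reference and starts looping Movement and Attack timers at their configured intervals.
; Movement and Attack are empty events, apparently hooks for child enemies to implement.
; AnyDamage subtracts from Health and destroys the actor at zero or below.
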(event `StartMovementTimer`
  ;[1 1 1] Movement
  (bind _returnvalue (`KismetSystemLibrary.K2_SetTimerDelegate` (delegate `Movement`) (`self.MovementSpeed`) true))
  (set `self.MovementTimerVariable` _returnvalue))

(event `StartAttackTimer`
  ;[1 1 1] Attacking
  (bind _returnvalue (`KismetSystemLibrary.K2_SetTimerDelegate` (delegate `Attack`) (`self.AttackTime`) true))
  (set `self.AttackTimerVariable` _returnvalue))

(event `self.DetectionSphere.OnComponentBeginOverlap`
  (params (OverlappedComponent :type "PrimitiveComponent Object Reference") (OtherActor :type "Actor Object Reference") (OtherComp :type "PrimitiveComponent Object Reference") (OtherBodyIndex :type Integer) (bFromSweep :type Boolean) (SweepResult :type "HitResult Structure (by ref)"))
  ;[1 1 1] Detection
  (bind _asbp_first_person_character (cast `/Game/FirstPerson/Blueprints/BP_FirstPersonCharacter` OtherActor))
  (set `self.Player` _asbp_first_person_character)
  (`self.StartMovementTimer`)
  (`self.StartAttackTimer`))

(event `Attack`
  ;[1 1 1] Attacking
)

(event `Movement`
  ;[1 1 1] Movement
)

(event `self.ReceiveAnyDamage`
  (params (Damage :type "Float (single-precision)") (DamageType :type "DamageType Object Reference") (InstigatedBy :type "Controller Object Reference") (DamageCauser :type "Actor Object Reference"))
  ;[1 1 1] Damage
  (bind _output_get (set `self.Health` (- (`self.Health`) Damage)))
  (if (<= _output_get 0.0)
    (`self.K2_DestroyActor`)))

(fn `UserConstructionScript`)